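; Base enemy character Blueprint with a montage-driven attack and a ledge-hang move.
; Construction places the actor slightly above the transform of its InitialLocation reference.
; Attack plays a montage and signals attack end on completion or interruption.
; HangOnLedge starts a looping ledge-surface check, moves the capsule to an offset facing into the ledge, and switches movement to Flying if not falling.
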(event `self.ReceiveBeginPlay`)

(event `Attack`
  (`|PlayMontage` (`self.Mesh`) "/Game/Characters/Mannequins/Anims/Unarmed/Attack/MM_Attack_01_Montage.MM_Attack_01_Montage"
    (:`OnCompleted`
      _)
    (:`OnInterrupted`
      _))
  (`self.OnAttackEnd`))

(fn `UserConstructionScript`
  (bind _returnvalue (`SceneComponent.K2_GetComponentToWorld` (`/Game/GameContent/GameGameplay/BP_InitialLocation.DefaultSceneRoot` (`self.InitialLocation`))))
  (`self.K2_SetActorTransform` (`KismetMathLibrary.MakeTransform` (`KismetMathLibrary.MakeVector` (.x (.location _returnvalue)) (.y (.location _returnvalue)) (+ (.z (.location _returnvalue)) 120.0)) (.rotation _returnvalue) (.scale _returnvalue))))