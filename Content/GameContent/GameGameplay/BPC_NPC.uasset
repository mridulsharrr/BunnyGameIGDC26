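; NPC character Blueprint with a placeholder world interaction that only prints a debug message, plus a ledge-hang function.
; HangOnLedge quickly moves the capsule below and out from the ledge along its normal, rotated to face it.
; It also starts a looping CheckIfLedgeHasSurface timer, whose function is not defined here, and switches movement to Flying if the character is not falling.
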(event `self.ReceiveBeginPlay`)

(event `/Game/GameContent/GameData/BPI_Interaction.WorldInteraction`
  (`KismetSystemLibrary.PrintString` "Interact"))

(fn `UserConstructionScript`)