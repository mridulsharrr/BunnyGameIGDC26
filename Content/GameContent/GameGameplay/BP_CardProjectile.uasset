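; BP_CardProjectile is a card projectile that flies toward an optional target and triggers a short-lived physics field on impact.
; The construction script applies gravity and speed to ProjectileMovement and enables homing on the target's root when IsHoming is set.
; BeginPlay aims velocity at any valid target.
; A Box hit spawns FS_MasterField at the hit actor, passes DamageMagnitude as radial magnitude, triggers it and destroys the projectile.
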(event `RotateToTarget`
  (set `MovementComponent.Velocity` (* (`KismetMathLibrary.GetDirectionUnitVector` (`self.K2_GetActorLocation`) (`self.K2_GetActorLocation` (`self.Target`))) (`self.Speed`)) (`self.ProjectileMovement`)))

(event `self.ReceiveBeginPlay`
  (`self.Target`
    (:`then`
      (`self.RotateToTarget`))
    (:`else`)))

(event `self.Box.OnComponentHit`
  (params (HitComponent :type "PrimitiveComponent Object Reference") (OtherActor :type "Actor Object Reference") (OtherComp :type "PrimitiveComponent Object Reference") (NormalImpulse :type "Vector Structure") (Hit :type "HitResult Structure (by ref)"))
  (bind (_returnvalue_location _returnvalue_rotation) (`KismetMathLibrary.BreakTransform` (`self.GetTransform` OtherActor)))
  (bind _returnvalue (`|SpawnActorFromClass` "/Engine/EditorResources/FieldNodes/FS_MasterField.FS_MasterField_C" (`KismetMathLibrary.MakeTransform` _returnvalue_location _returnvalue_rotation (* (1.0 1.0 1.0) 1.0)) "Undefined" "MultiplyWithRoot" null null))
  (set `/Engine/EditorResources/FieldNodes/FS_MasterField.Radial Magnitude` (`self.Damage Magnitude`) _returnvalue)
  (set `/Engine/EditorResources/FieldNodes/FS_MasterField.FieldLifespan` 0.2 _returnvalue)
  (set `/Engine/EditorResources/FieldNodes/FS_MasterField.ActivationType` "NewEnumerator4" _returnvalue)
  (`/Engine/EditorResources/FieldNodes/FS_MasterField.CE_Trigger` _returnvalue)
  (`self.K2_DestroyActor`))

(fn `UserConstructionScript`
  (bind _projectilemovement (`self.ProjectileMovement`))
  (bind _speed (`self.Speed`))
  (bind _projectilemovement_2 (`self.ProjectileMovement`))
  (set `ProjectileMovementComponent.ProjectileGravityScale` (`self.Gravity`) _projectilemovement)
  (set `ProjectileMovementComponent.InitialSpeed` _speed _projectilemovement)
  (set `ProjectileMovementComponent.MaxSpeed` _speed _projectilemovement)
  (`self.Target`
    (:`then`
      (if (`self.isHoming`)
        (set `ProjectileMovementComponent.bIsHomingProjectile` true _projectilemovement_2)
        (set `ProjectileMovementComponent.HomingTargetComponent` (`Actor.RootComponent` (`self.Target`)) _projectilemovement_2)))
    (:`else`)))