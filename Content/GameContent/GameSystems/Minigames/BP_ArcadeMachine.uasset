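; Interactable arcade machine that plays a media source and hands the player over to a minigame.
; The media player opens and plays on construction and at BeginPlay.
; On interaction, it fades the camera, hides the player character, possesses the existing BP_MiniGame and sets the view target to the cabinet.
; The minigame's UpdateOffset event tilts the cabinet's joystick left, center or right.
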(event `self.ReceiveBeginPlay`
  (bind _mediaplayer (`self.MediaPlayer`))
  (`MediaPlayer.OpenSource` _mediaplayer (`self.Media Source`))
  (`MediaPlayer.Play` _mediaplayer))

(event `CustomEvent`
  (params (Var :type Integer))
  (bind _joystick (`self.Joystick`))
  (switch `int` Var
    (:`-1`
      (`SceneComponent.K2_SetRelativeRotation` (`self.Joystick`) (struct :`Pitch` -13.452303) false false))
    (:`0`
      (`SceneComponent.K2_SetRelativeRotation` :`self` _joystick))
    (:`1`
      (`SceneComponent.K2_SetRelativeRotation` _joystick (struct :`Pitch` 13.452303) false false))))

(event `/Game/GameContent/GameData/BPI_Interaction.Interaction`
  (params (Interactor :type "Actor Object Reference"))
  (bind _returnvalue (`GameplayStatics.GetActorOfClass` "/Game/GameContent/GameSystems/Minigames/BP_MiniGame.BP_MiniGame_C"))
  (add `/Game/GameContent/GameSystems/Minigames/BP_MiniGame.Update Offset` _returnvalue (delegate `CustomEvent`))
  (`PlayerCameraManager.StartCameraFade` :`self` (`GameplayStatics.GetPlayerCameraManager` 0) :`ToAlpha` 1.0 :`Duration` 0.5 :`bHoldWhenFinished` true)
  (`KismetSystemLibrary.Delay` 0.6)
  (`self.SetActorHiddenInGame` (`GameplayStatics.GetPlayerCharacter` 0) true)
  (`Controller.Possess` (`GameplayStatics.GetPlayerController` 0) _returnvalue)
  (`PlayerCameraManager.StartCameraFade` :`self` (`GameplayStatics.GetPlayerCameraManager` 0) :`FromAlpha` 1.0 :`Duration` 0.5 :`bHoldWhenFinished` true)
  (`PlayerController.SetViewTargetWithBlend` (`GameplayStatics.GetPlayerController` 0) self 0.0 "VTBlend_Linear" 0.0 false))

(fn `UserConstructionScript`
  (bind _mediaplayer (`self.MediaPlayer`))
  (`MediaPlayer.OpenSource` _mediaplayer (`self.Media Source`))
  (`MediaPlayer.Play` _mediaplayer))