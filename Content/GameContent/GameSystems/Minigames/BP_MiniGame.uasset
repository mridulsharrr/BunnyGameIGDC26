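; Three-lane dodge minigame in which the player shifts sideways while an enemy slides toward them.
; Left and right inputs step the Player component between lanes and call UpdateOffset with the direction, zeroed on release.
; MoveEnemy respawns the Enemy in a random lane, and a looping timer advances it, speeding up to a cap as crossings accumulate.
; E fades the screen and returns possession and view to BPC_Rabbit.
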(event `Key|Gamepad_DPad_Right`
  (params (Key :type "Key Structure"))
  (bind _player (`self.Player`))
  (bind (_relativelocation_x _relativelocation_y _relativelocation_z) (`KismetMathLibrary.BreakVector` (`SceneComponent.RelativeLocation` _player)))
  (:`Pressed`
    (`|ExecutionSequence` :!label _label
      (:`then_0`
        (switch `int` (`self.positionInt`)
          (:`0`
            (set `self.positionInt` 0 :!label _label_2)
            (`SceneComponent.K2_SetRelativeLocation` (`self.Player`) (`KismetMathLibrary.MakeVector` _relativelocation_x -100.0 _relativelocation_z) false false))
          (:`1`
            (goto _label_2))
          (:`2`
            (set `self.positionInt` 1)
            (`SceneComponent.K2_SetRelativeLocation` _player (`KismetMathLibrary.MakeVector` _relativelocation_x 0.0 _relativelocation_z) false false :!label _label_3))))
      (:`then_1`
        (`self.Update Offset` (`KismetMathLibrary.FTrunc` -1.0)))))
  (:`Released`
    (`self.Update Offset` 0 :!label _label_4)))

(event `Key|D`
  (params (Key :type "Key Structure"))
  (:`Pressed`
    (goto _label))
  (:`Released`
    (goto _label_4)))

(event `Key|Right`
  (params (Key :type "Key Structure"))
  (:`Pressed`
    (goto _label))
  (:`Released`
    (goto _label_4)))

(event `Key|Gamepad_DPad_Left`
  (params (Key :type "Key Structure"))
  (bind _player (`self.Player`))
  (bind (_relativelocation_x _relativelocation_y _relativelocation_z) (`KismetMathLibrary.BreakVector` (`SceneComponent.RelativeLocation` _player)))
  (:`Pressed`
    (`|ExecutionSequence` :!label _label_5
      (:`then_0`
        (switch `int` (`self.positionInt`)
          (:`0`
            (set `self.positionInt` 1)
            (goto _label_3))
          (:`1`
            _)
          (:`2`
            _))
        (set `self.positionInt` 2)
        (`SceneComponent.K2_SetRelativeLocation` _player (`KismetMathLibrary.MakeVector` _relativelocation_x 100.0 _relativelocation_z) false false))
      (:`then_1`
        (`self.Update Offset` (`KismetMathLibrary.FTrunc` 1.0)))))
  (:`Released`
    (goto _label_4)))

(event `Key|A`
  (params (Key :type "Key Structure"))
  (:`Pressed`
    (goto _label_5))
  (:`Released`
    (goto _label_4)))

(event `Key|Left`
  (params (Key :type "Key Structure"))
  (:`Pressed`
    (goto _label_5))
  (:`Released`
    (goto _label_4)))

(event `Key|E`
  (params (Key :type "Key Structure"))
  (:`Pressed`
    (bind _returnvalue (`GameplayStatics.GetActorOfClass` "/Game/GameContent/GameGameplay/BPC_Rabbit.BPC_Rabbit_C"))
    (`PlayerCameraManager.StartCameraFade` :`self` (`GameplayStatics.GetPlayerCameraManager` 0) :`ToAlpha` 1.0 :`Duration` 0.5 :`bHoldWhenFinished` true)
    (`KismetSystemLibrary.Delay` 0.6)
    (`self.SetActorHiddenInGame` _returnvalue false)
    (`Controller.Possess` (`GameplayStatics.GetPlayerController` 0) _returnvalue)
    (`PlayerCameraManager.StartCameraFade` :`self` (`GameplayStatics.GetPlayerCameraManager` 0) :`FromAlpha` 1.0 :`Duration` 0.5 :`bHoldWhenFinished` true)
    (`PlayerController.SetViewTargetWithBlend` (`GameplayStatics.GetPlayerController` 0) _returnvalue 0.0 "VTBlend_Linear" 0.0 false)))

(event `Move Enemy`
  (bind _output_get (set `self.enemyposInt` (`KismetMathLibrary.RandomIntegerInRange` 0 2)))
  (`SceneComponent.K2_SetRelativeLocation` (`self.Enemy`) (`KismetMathLibrary.MakeVector` 699.647117 (select `int` _output_get :`0` -100.0 :`1` 0.0 :`2` 100.0) 43.64053) false false)
  (`self.StartMove`))

(event `StartMove`
  (bind _crossedindex (`self.crossedIndex`))
  (set `self.Speed` (`KismetMathLibrary.SelectFloat` -22.0 (select `int` _crossedindex :`0` -4.0 :`1` -8.0 :`2` -10.0 :`3` -13.0 :`4` -17.0) (> _crossedindex 4)))
  (`KismetSystemLibrary.K2_SetTimerDelegate` (delegate `CustomEvent`) 0.1 true))

(event `CustomEvent`
  (bind (_relativelocation_x _relativelocation_y _relativelocation_z) (`KismetMathLibrary.BreakVector` (`SceneComponent.RelativeLocation` (`self.Enemy`))))
  (`SceneComponent.K2_SetRelativeLocation` (`self.Enemy`) (`KismetMathLibrary.MakeVector` (+ _relativelocation_x (`self.Speed`)) _relativelocation_y _relativelocation_z) true false)
  (if (<= _relativelocation_x -160.0)
    (bind _result (`/Engine/EditorBlueprintResources/StandardMacros.IncrementInt` (`self.crossedIndex`))
      (:`  `
        (set `self.crossedIndex` _result)
        (`self.Move Enemy`)))))

(fn `UserConstructionScript`)