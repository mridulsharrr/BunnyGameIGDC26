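; BP_MainInstance is the game instance that owns the game's main save and holds debug stat toggles.
; On Init it loads the MainSlot save if one exists, otherwise it creates and writes a new one, caching the object in SaveGame.
; Separate events delete that slot and store the StatFPS and StatGPU values.
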(event `/Game/GameContent/GameSystems/BPI_Dev.Stats`
  (params (`Stat FPS` :type Boolean) (`Stat GPU` :type Boolean))
  (set `self.Stat FPS` `Stat FPS`)
  (set `self.Stat GPU` `Stat GPU`))

(event `self.ReceiveInit`
  (bind _returnvalue (`GameplayStatics.DoesSaveGameExist` (`self.MainSlot`)))
  (if _returnvalue
    (bind _returnvalue_2 (`GameplayStatics.LoadGameFromSlot` (`self.MainSlot`)))
    (set `self.SaveGame` _returnvalue_2)
    (else
      (bind _returnvalue_3 (`GameplayStatics.CreateSaveGameObject` "/Script/Engine.SaveGame"))
      (`GameplayStatics.SaveGameToSlot` _returnvalue_3 (`self.MainSlot`))
      (set `self.SaveGame` _returnvalue_3))))

(event `DeleteSave`
  (`GameplayStatics.DeleteGameInSlot` (`self.MainSlot`)))